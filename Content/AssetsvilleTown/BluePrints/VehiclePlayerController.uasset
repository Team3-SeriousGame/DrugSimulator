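; Player controller for a drivable wheeled vehicle that sets up input and a vehicle HUD.
; BeginPlay adds an Enhanced Input mapping context, creates the HUD widget and caches the controlled pawn's vehicle movement component.
; Tick reads forward speed and current gear from that component and passes them to UpdateSpeed and UpdateGear calls.
; The controller's own UpdateSpeed event and function are empty stubs.
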(event `self.ReceiveBeginPlay`
  (`EnhancedInputSubsystemInterface.AddMappingContext` (subsystem `EnhancedInputLocalPlayerSubsystem`) null 0 (struct)) ; Adding the Input Mapping Context needed to trigger the proper Input Actions.
  (bind _returnvalue (`|GenericCreateObject` self null))
  (set `self.VehicleHud` _returnvalue)
  (`UserWidget.AddToViewport` 0)
  (bind _aswheeled_vehicle_pawn (cast `WheeledVehiclePawn` (`self.K2_GetPawn`)))
  (set `self.Vehicle Movement Component` (`WheeledVehiclePawn.VehicleMovementComponent` _aswheeled_vehicle_pawn)))

(event `self.ReceiveTick`
  (params (DeltaSeconds :type "Float (single-precision)"))
  (`self.UpdateSpeed` (`ChaosVehicleMovementComponent.GetForwardSpeed` (`self.Vehicle Movement Component`)))
  (`self.UpdateGear` (`ChaosVehicleMovementComponent.GetCurrentGear` (`self.Vehicle Movement Component`))))

(event `UpdateSpeed`
  (params (NewSpeed :type "Float (double-precision)")))

(fn `Update Speed`)

(fn `UserConstructionScript`)